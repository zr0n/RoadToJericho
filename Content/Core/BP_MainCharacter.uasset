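; Player character for a Temple Run-style game, adding a cross-sphere backdrop and a cinematic death sequence to its parent class.
; The sphere follows the character on X only, while a self-restarting timeline animates its material inversion.
; On the game mode's game over, the mesh ragdolls and the detached camera glides to a reference point, turning toward the sphere.
; Wings, lights and game-over UI then appear as the mesh stops simulating and flies upward.
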(event Custom|InvertColorFX
  (bind _alpha (Timeline|InvertColorFXTL PlayFromStart)
    (:Update
      (Rendering|Material|SetScalarParameterValueonMaterials (Variables|Default|GetCrossesSphere) "AlphaInvert" _alpha))
    (:Finished
      (CallFunction|InvertColorFX))))

(event Custom|SetupCross
  (bind _crossessphere (Variables|Default|GetCrossesSphere))
  (bind _returnvalue (Transformation|GetWorldLocation _crossessphere))
  (Utilities|FlowControl|Sequence
    (:then_0
      (Utilities|FlowControl|DoOnce false
        (:Completed
          (Transformation|SetAbsolute (Variables|Default|GetCrossesSphere) true true true)
          (Variables|Default|SetInitialCrossX (.x _returnvalue)))))
    (:then_1
      (Transformation|SetWorldLocation _crossessphere (Math|Vector|MakeVector (+ (.x (Transformation|GetActorLocation)) (Variables|Default|GetInitialCrossX)) (.y _returnvalue) (.z _returnvalue)) false false))))

(event Custom|BindGameOver
  (EventDispatchers|AssignOnGameOver (Variables|Default|GetGM) (delegate Custom|OnGameOver)))

(event Custom|OnGameOver
  (bind _mesh (Variables|Character|GetMesh))
  (bind _mesh_2 (Variables|Character|GetMesh))
  (bind _camera (Variables|Default|GetCamera))
  (Utilities|Time|SetTimerbyEvent (delegate Custom|FixCamera) 0.01 true)
  (Utilities|FlowControl|DoOnce false
    (:Completed
      (Collision|SetCollisionEnabled (Variables|Character|GetMesh) "PhysicsOnly")
      (Utilities|FlowControl|Delay 0.1)
      (Physics|SetSimulatePhysics _mesh_2 true)
      (Class|SkeletalMeshComponent|SetAllBodiesBelowSimulatePhysics _mesh_2 (Class|SkinnedMeshComponent|GetBoneName _mesh_2) true true)
      (Utilities|FlowControl|Delay 0.8)
      (Transformation|DetachFromComponent (Variables|Default|GetCamera) "KeepWorld" "KeepWorld" "KeepWorld" true)
      (Variables|/Script/Engine.SceneComponent|SetbAbsoluteLocation (Variables|Default|GetCamera) true)
      (Variables|Default|SetOldLocation (Transformation|GetWorldLocation (Variables|Default|GetCamera)))
      (Variables|/Script/Engine.SpringArmComponent|SetbEnableCameraLag (Variables|Default|GetSpringArm) false)
      (Variables|Default|SetDesiredLocation (Transformation|GetWorldLocation (Variables|Default|GetCameraReference)))
      (bind _alpha (Timeline|SetCameraTL PlayFromStart)
        (:Update
          (Transformation|SetWorldLocation (Variables|Default|GetCamera) (Math|Vector|Lerp(Vector) (Variables|Default|GetOldLocation) (Variables|Default|GetDesiredLocation) _alpha) true true)
          (Transformation|SetWorldRotation _camera (Math|Rotator|Lerp(Rotator) (Transformation|GetWorldRotation _camera) (Math|Rotator|FindLookatRotation (Transformation|GetWorldLocation _camera) (Transformation|GetWorldLocation (Variables|Default|GetCrossesSphere))) (* (Variables|Default|GetDeathCameraSmoothFactor) (Utilities|Time|GetWorldDeltaSeconds)) true) false false))
        (:Finished
          (Variables|Default|SetFinishedAnimation true)
          (Rendering|SetVisibility (Variables|Default|GetWings) true false)
          (CallFunction|GameOverUI)
          (Utilities|FlowControl|Sequence
            (:then_0
              (bind _alpha_2 (Timeline|Timeline_0 PlayFromStart)
                (:Update
                  (Rendering|Components|Light|SetIntensity (Variables|Default|GetSpotLight) (Math|Float|Lerp 1e+08 1e+09 _alpha_2))
                  (Rendering|Components|Light|SetLightColor (Variables|Default|GetSpotLight) (Math|Color|Lerp(LinearColor) "(R=1.000000,G=0.015686,B=0.000000,A=1.000000)" "(R=1.000000,G=0.501961,B=0.000000,A=1.000000)" _alpha_2) true))))
            (:then_1
              (Physics|SetSimulatePhysics (Variables|Character|GetMesh) false)
              (Rendering|SetVisibility (Variables|Default|GetPointLight1) true false)
              (Transformation|SetAbsolute _mesh false true false)
              (Class|SkeletalMeshComponent|SetAllBodiesBelowSimulatePhysics _mesh (Class|SkinnedMeshComponent|GetBoneName _mesh) false true)
              (Transformation|SetWorldRotation _mesh (Transformation|GetWorldRotation (Variables|Default|GetReference2)) false false)
              (Transformation|SetWorldScale3D (Variables|Character|GetMesh) (Math|Vector|MakeVector 0.8 0.8 0.8))
              (Transformation|AttachComponentToComponent (Variables|Character|GetMesh) (Variables|Default|GetReference1) "None" "KeepWorld" "KeepWorld" "KeepWorld" false)
              (bind _alpha_3 (Timeline|FlyUp PlayFromStart)
                (:Update
                  (Transformation|SetWorldLocation (Variables|Character|GetMesh) (Math|Vector|Lerp(Vector) (Transformation|GetWorldLocation (Variables|Default|GetReference2)) (Transformation|GetWorldLocation (Variables|Default|GetReference1)) _alpha_3) false true))
                (:Finished
                  (Variables|Default|SetFinishedFlyUpAnimation true))))))))))

(event Custom|GameOverUI
  (bind _returnvalue (UserInterface|CreateWidget "/Game/UI/UI_GameOver.UI_GameOver_C"))
  (UserInterface|Viewport|AddtoViewport _returnvalue 0))

(event Custom|FixCamera
  (bind _camera (Variables|Default|GetCamera))
  (if (Variables|Default|GetFinishedAnimation)
    (Transformation|SetWorldRotation _camera (Math|Rotator|Lerp(Rotator) (Transformation|GetWorldRotation _camera) (Math|Rotator|FindLookatRotation (Transformation|GetWorldLocation _camera) (Transformation|GetWorldLocation (Variables|Default|GetCrossesSphere))) (* (Variables|Default|GetDeathCameraSmoothFactor) (Utilities|Time|GetWorldDeltaSeconds)) true) false false)))

(event EventBeginPlay
  (|CallParentFunction)
  (CallFunction|InvertColorFX)
  (bind _astemple_run_game_mode_base (Utilities|Casting|CastToTempleRunGameModeBase (Game|GetGameMode)))
  (Variables|Default|SetGM _astemple_run_game_mode_base)
  (CallFunction|BindGameOver))

(event EventTick
  (params (DeltaSeconds :type Float%20%28single-precision%29))
  (|CallParentFunction DeltaSeconds)
  (CallFunction|SetupCross)
  (Utilities|IsValid (Variables|Default|GetGM)
    (:Is%20Valid
      (if (Variables|Default|GetFinishedFlyUpAnimation)
        _))))

(fn ConstructionScript)