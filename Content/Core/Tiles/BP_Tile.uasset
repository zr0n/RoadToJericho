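; BP_Tile is a floor tile for a Temple Run-style game, with a destructible floor that breaks apart.
; When the main character overlaps SpawnTrigger, it shakes the camera, plays rock-falling audio and fractures the floor with randomized radius damage.
; On game over, it disables cube collision, waits briefly at random, enables floor physics and applies the same damage.
; Tiles that begin play after the match ends destroy themselves.
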(event OnComponentBeginOverlap(SpawnTrigger)
  (params (OverlappedComponent :type Primitive%20Component%20Object%20Reference) (OtherActor :type Actor%20Object%20Reference) (OtherComp :type Primitive%20Component%20Object%20Reference) (OtherBodyIndex :type Integer) (bFromSweep :type Boolean) (SweepResult :type Hit%20Result%20Structure%20%28by%20ref%29))
  (bind _asbp_main_character (Utilities|Casting|CastToBP_MainCharacter OtherActor))
  (CallFunction|CameraShake _asbp_main_character)
  (CallFunction|PlayAudio)
  (Class|DestructibleComponent|ApplyRadiusDamage (Variables|Default|GetFloorDestructible) (Math|Random|RandomFloatinRange 3e+02 9e+02) (Transformation|GetActorLocation) (Math|Random|RandomFloatinRange 3e+02 8e+02) (Math|Random|RandomFloatinRange 1.5e+03 5e+03) true))

(event Custom|OnGameOver
  (Collision|SetCollisionEnabled (Variables|Default|GetCube) "NoCollision")
  (Utilities|FlowControl|Delay (Math|Random|RandomFloatinRange 0.0 0.3))
  (Physics|SetSimulatePhysics (Variables|Default|GetFloorDestructible) true)
  (Class|DestructibleComponent|ApplyRadiusDamage (Variables|Default|GetFloorDestructible) (Math|Random|RandomFloatinRange 3e+02 9e+02) (Transformation|GetActorLocation) (Math|Random|RandomFloatinRange 3e+02 8e+02) (Math|Random|RandomFloatinRange 1.5e+03 5e+03) true))

(event Custom|PlayAudio
  (Audio|PlaySoundatLocation "/Game/Audio/RockFalling_Cue.RockFalling_Cue" (Transformation|GetWorldLocation (Variables|Default|GetSpawnTrigger)) "0, 0, 0" 0.5 1.0 0.0 "/Game/Audio/RockAttenuation.RockAttenuation" 0 0))

(event Custom|CameraShake
  (params (As%20Base%20Character :type BP%20Main%20Character%20Object%20Reference))
  (Camera|PlayWorldCameraShake "/Game/Misc/GroundBreakShake.GroundBreakShake_C" (Transformation|GetWorldLocation (Variables|/Game/Core/BP_MainCharacter.BP_MainCharacter_C|GetCamera As%20Base%20Character)) 3e+02 5e+02 1.0 true))

(event EventBeginPlay
  (|CallParentFunction)
  (bind _astemple_run_game_mode_base (Utilities|Casting|CastToTempleRunGameModeBase (Game|GetGameMode)))
  (if (Utilities|Name|NotEqual(Name) (Class|GameMode|GetMatchState _astemple_run_game_mode_base) "Over")
    (EventDispatchers|AssignOnGameOver _astemple_run_game_mode_base (delegate Custom|OnGameOver))
    (else
      (Actor|DestroyActor))))

(fn ConstructionScript)