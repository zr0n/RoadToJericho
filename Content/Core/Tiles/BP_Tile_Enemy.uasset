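; BP_Tile_Enemy is a tile Blueprint that carries an enemy as a child actor and switches it to physics simulation when triggered.
; Either game over or a BaseCharacter overlapping SpawnTrigger starts the same sequence, which waits a short random delay, then enables physics on the BP_Enemy mesh.
; A downward AddForce on that mesh is left unconnected and never runs.
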(event OnComponentBeginOverlap(SpawnTrigger)
  (params (OverlappedComponent :type Primitive%20Component%20Object%20Reference) (OtherActor :type Actor%20Object%20Reference) (OtherComp :type Primitive%20Component%20Object%20Reference) (OtherBodyIndex :type Integer) (bFromSweep :type Boolean) (SweepResult :type Hit%20Result%20Structure%20%28by%20ref%29))
  (Utilities|Casting|CastToBaseCharacter OtherActor)
  (bind _asbp_enemy (Utilities|Casting|CastToBP_Enemy (Variables|/Script/Engine.ChildActorComponent|GetChildActor (Variables|Default|GetEnemy_Child))))
  (Utilities|FlowControl|Delay (Math|Random|RandomFloatinRange 0.3 0.5))
  (Physics|SetSimulatePhysics (Variables|/Script/TempleRun.Enemy|GetMesh _asbp_enemy) true))

(event EventBeginPlay
  (|CallParentFunction))

(event Collision|EventActorBeginOverlap
  (params (OtherActor :type Actor%20Object%20Reference))
  (|CallParentFunction OtherActor) ; This node is disabled and will not be called.\nDrag off pins to build functionality.
)

(event EventTick
  (params (DeltaSeconds :type Float%20%28single-precision%29))
  (|CallParentFunction DeltaSeconds) ; This node is disabled and will not be called.\nDrag off pins to build functionality.
)

(event EventOnGameOver
  (|CallParentFunction)
  (bind _asbp_enemy (Utilities|Casting|CastToBP_Enemy (Variables|/Script/Engine.ChildActorComponent|GetChildActor (Variables|Default|GetEnemy_Child))))
  (Utilities|FlowControl|Delay (Math|Random|RandomFloatinRange 0.3 0.5))
  (Physics|SetSimulatePhysics (Variables|/Script/TempleRun.Enemy|GetMesh _asbp_enemy) true))

(fn ConstructionScript
  (|CallParentFunction))