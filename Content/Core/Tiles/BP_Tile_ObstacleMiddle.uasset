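; Middle obstacle tile for a temple runner that ends the game when the player character touches the obstacle.
; A random yaw varies it at start, and a Tick distance check fades it in once through a timeline-driven "Amount" material parameter.
; The spawn trigger makes it fall away with physics, random delay and torque.
; Game over reuses that tumble and plays the fade timeline in reverse.
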(event OnComponentBeginOverlap(Obstacle)
  (params (OverlappedComponent :type Primitive%20Component%20Object%20Reference) (OtherActor :type Actor%20Object%20Reference) (OtherComp :type Primitive%20Component%20Object%20Reference) (OtherBodyIndex :type Integer) (bFromSweep :type Boolean) (SweepResult :type Hit%20Result%20Structure%20%28by%20ref%29))
  (if (Utilities|ClassIsChildOf (Utilities|GetClass OtherActor) "/Script/TempleRun.BaseCharacter")
    (bind _astemple_run_game_mode_base (Utilities|Casting|CastToTempleRunGameModeBase (Game|GetGameMode)))
    (Class|TempleRunGameModeBase|GameOver _astemple_run_game_mode_base)))

(event OnComponentBeginOverlap(SpawnTrigger)
  (params (OverlappedComponent :type Primitive%20Component%20Object%20Reference) (OtherActor :type Actor%20Object%20Reference) (OtherComp :type Primitive%20Component%20Object%20Reference) (OtherBodyIndex :type Integer) (bFromSweep :type Boolean) (SweepResult :type Hit%20Result%20Structure%20%28by%20ref%29))
  (bind _obstacle (Variables|Default|GetObstacle))
  (Utilities|Casting|CastToBaseCharacter OtherActor)
  (Utilities|FlowControl|Delay (Math|Random|RandomFloatinRange 0.0 0.3))
  (Physics|SetSimulatePhysics _obstacle true)
  (Physics|AddForce _obstacle (* (Transformation|GetActorUpVector) -6e+01) "None" true)
  (Utilities|FlowControl|Delay 0.2)
  (Class|PrimitiveComponent|AddTorqueinDegrees _obstacle (Math|Vector|MakeVector (Math|Random|RandomFloatinRange 1e+02 2e+02) (Math|Random|RandomFloatinRange 1e+02 2e+02) (Math|Random|RandomFloatinRange 1e+02 2e+02)) "None" true))

(event Custom|Appear
  (bind _alphaappear (Timeline|AppearTL PlayFromStart)
    (:Update
      (Rendering|Material|SetScalarParameterValueonMaterials (Variables|Default|GetObstacle) "Amount" _alphaappear))
    (:Finished
      (Variables|Default|SetObstacleOnScreen true))))

(event Custom|CheckAppear
  (if (and (<= (Transformation|GetDistanceTo (Variables|Default|GetCharacter) self) (Variables|Default|GetOffsetToShowObstacle)) (not (Variables|Default|GetObstacleOnScreen)))
    (Utilities|FlowControl|DoOnce false
      (:Completed
        (CallFunction|Appear)))))

(event Custom|RandomRotationDeviation
  (Transformation|AddRelativeRotation (Variables|Default|GetObstacle) (Math|Rotator|MakeRotator 0.0 0.0 (Math|Float|Lerp (Variables|Default|GetMinRotationZ) (Variables|Default|GetMaxRotationZ) (Math|Random|RandomFloat))) false false))

(event EventBeginPlay
  (|CallParentFunction)
  (Variables|Default|SetCharacter (Game|GetPlayerCharacter 0))
  (Rendering|Material|SetScalarParameterValueonMaterials (Variables|Default|GetObstacle) "Amount" 1.0)
  (CallFunction|RandomRotationDeviation))

(event EventTick
  (params (DeltaSeconds :type Float%20%28single-precision%29))
  (CallFunction|CheckAppear))

(event EventOnGameOver
  (bind _obstacle (Variables|Default|GetObstacle))
  (|CallParentFunction)
  (Utilities|FlowControl|Sequence
    (:then_0
      (Utilities|FlowControl|Delay (Math|Random|RandomFloatinRange 0.0 0.3))
      (Physics|SetSimulatePhysics _obstacle true)
      (Physics|AddForce _obstacle (* (Transformation|GetActorUpVector) -6e+01) "None" true)
      (Utilities|FlowControl|Delay 0.2)
      (Class|PrimitiveComponent|AddTorqueinDegrees _obstacle (Math|Vector|MakeVector (Math|Random|RandomFloatinRange 1e+02 2e+02) (Math|Random|RandomFloatinRange 1e+02 2e+02) (Math|Random|RandomFloatinRange 1e+02 2e+02)) "None" true))
    (:then_1
      (bind _alphaappear (Timeline|AppearTL ReverseFromEnd)
        (:Update
          (Rendering|Material|SetScalarParameterValueonMaterials (Variables|Default|GetObstacle) "Amount" _alphaappear))
        (:Finished
          (Variables|Default|SetObstacleOnScreen true))))))

(fn ConstructionScript
  (|CallParentFunction)
  (Rendering|Material|SetScalarParameterValueonMaterials (Variables|Default|GetObstacle) "Amount" (Variables|Default|GetAlpha)))