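; BP_BoxMask1 is an animated box mask actor that feeds its cube's transform to materials, apparently for the EasyDissolve effect.
; Tick writes world location, scale times 100 and rotation normalized by 360 into the second box slot of MPC_BoxMask.
; BeginPlay runs a timeline that scales the cube and triggers another that rotates it.
; A one-second Delay on Tick then plays a timeline driving the cube's Opacity material parameter.
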(event EventBeginPlay
  (bind _cube (Variables|Default|GetCube))
  (bind _newtrack_0 (Timeline|Timeline_0 Play)
    (:Update
      (Transformation|SetWorldScale3D _cube _newtrack_0)
      (bind _newtrack_0_2 (Timeline|Timeline_1 Play)
        (:Update
          (Transformation|SetWorldRotation _cube (Math|Rotator|MakeRotator _newtrack_0_2 (* _newtrack_0_2 45.0) (* _newtrack_0_2 6e+01)) false false))))))

(event EventTick
  (params (DeltaSeconds :type Float%20%28single-precision%29))
  (bind _cube (Variables|Default|GetCube))
  (bind _returnvalue (Transformation|GetWorldRotation _cube))
  (bind (_roll _pitch _yaw) (Math|Rotator|BreakRotator _returnvalue))
  (Rendering|Material|SetVectorParameterValue "/Game/EasyDissolve/Materials/CollectionParameters/MPC_BoxMask.MPC_BoxMask" "BoxBounds_2" (Math|Conversions|ToLinearColor(Vector) (* (Transformation|GetWorldScale _cube) 1e+02)) :!class /Script/Engine.KismetMaterialLibrary)
  (Rendering|Material|SetVectorParameterValue "/Game/EasyDissolve/Materials/CollectionParameters/MPC_BoxMask.MPC_BoxMask" "Location_2" (Math|Conversions|ToLinearColor(Vector) (Transformation|GetWorldLocation _cube)) :!class /Script/Engine.KismetMaterialLibrary)
  (Rendering|Material|SetVectorParameterValue "/Game/EasyDissolve/Materials/CollectionParameters/MPC_BoxMask.MPC_BoxMask" "Rotation_2" (Math|Conversions|ToLinearColor(Vector) (Math|Vector|MakeVector (/ _roll 3.6e+02) (/ _pitch 3.6e+02) (/ _yaw 3.6e+02))) :!class /Script/Engine.KismetMaterialLibrary)
  (Utilities|FlowControl|Delay 1.0)
  (bind _newtrack_0 (Timeline|Timeline_2 Play)
    (:Update
      (Rendering|Material|SetScalarParameterValueonMaterials (Variables|Default|GetCube) "Opacity" _newtrack_0))))

(fn ConstructionScript)