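; BP_BoxMask is a box mask actor for a dissolve effect, feeding a cube's transform to materials through MPC_BoxMask.
; Every tick it writes the cube's scaled bounds, location and normalized rotation to the collection's first box slot.
; From BeginPlay, a Scale timeline resizes the cube and starts a Rotation timeline that spins it.
; An Opacity timeline, played from Tick, drives the cube materials' opacity.
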(event EventBeginPlay
  (bind _cube (Variables|Default|GetCube))
  (bind _newtrack_0 (Timeline|Scale Play)
    (:Update
      (Transformation|SetWorldScale3D _cube _newtrack_0)
      (bind _newtrack_0_2 (Timeline|Rotation Play)
        (:Update
          (Transformation|SetWorldRotation _cube (Math|Rotator|MakeRotator _newtrack_0_2 (* _newtrack_0_2 1.8e+02) (* _newtrack_0_2 9e+01)) false false))))))

(event EventTick
  (params (DeltaSeconds :type Float%20%28single-precision%29))
  (bind _cube (Variables|Default|GetCube))
  (bind _returnvalue (Transformation|GetWorldRotation _cube))
  (bind (_roll _pitch _yaw) (Math|Rotator|BreakRotator _returnvalue))
  (Rendering|Material|SetVectorParameterValue "/Game/EasyDissolve/Materials/CollectionParameters/MPC_BoxMask.MPC_BoxMask" "BoxBounds_1" (Math|Conversions|ToLinearColor(Vector) (* (Transformation|GetWorldScale _cube) 1e+02)) :!class /Script/Engine.KismetMaterialLibrary)
  (Rendering|Material|SetVectorParameterValue "/Game/EasyDissolve/Materials/CollectionParameters/MPC_BoxMask.MPC_BoxMask" "Location_1" (Math|Conversions|ToLinearColor(Vector) (Transformation|GetWorldLocation _cube)) :!class /Script/Engine.KismetMaterialLibrary)
  (Rendering|Material|SetVectorParameterValue "/Game/EasyDissolve/Materials/CollectionParameters/MPC_BoxMask.MPC_BoxMask" "Rotation_1" (Math|Conversions|ToLinearColor(Vector) (Math|Vector|MakeVector (/ _roll 3.6e+02) (/ _pitch 3.6e+02) (/ _yaw 3.6e+02))) :!class /Script/Engine.KismetMaterialLibrary)
  (bind _newtrack_0 (Timeline|Opacity Play)
    (:Update
      (Rendering|Material|SetScalarParameterValueonMaterials (Variables|Default|GetCube) "Opacity" _newtrack_0))))

(fn ConstructionScript)