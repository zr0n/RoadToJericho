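; BP_SphereMask is an actor that feeds a sphere's position and size to the MPC_SphereMask material parameter collection, apparently driving EasyDissolve mask effects.
; Construction script and Tick write Location_1 from the sphere's world location and Radius_1 from its X scale times 50.
; BeginPlay plays a timeline that moves the root component.
; Tick also plays a second timeline that animates the sphere material's Opacity.
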(event EventBeginPlay
  (bind _newtrack_0 (Timeline|Timeline_0 Play)
    (:Update
      (Components|MoveComponentTo (Variables|Default|GetDefaultSceneRoot) _newtrack_0 "0, 0, 0" false false 0.2 false))))

(event Collision|EventActorBeginOverlap
  (params (OtherActor :type Actor%20Object%20Reference)))

(event EventTick
  (params (DeltaSeconds :type Float%20%28single-precision%29))
  (Rendering|Material|SetScalarParameterValue "/Game/EasyDissolve/Materials/CollectionParameters/MPC_SphereMask.MPC_SphereMask" "Radius_1" (.X (Math|Vector|BreakVector (* (/ (Transformation|GetWorldScale (Variables|Default|GetSphere)) 2.0) 1e+02))) :!class /Script/Engine.KismetMaterialLibrary)
  (Rendering|Material|SetVectorParameterValue "/Game/EasyDissolve/Materials/CollectionParameters/MPC_SphereMask.MPC_SphereMask" "Location_1" (Math|Conversions|ToLinearColor(Vector) (Transformation|GetWorldLocation (Variables|Default|GetSphere))) :!class /Script/Engine.KismetMaterialLibrary)
  (bind _newtrack_0 (Timeline|Timeline_1 Play)
    (:Update
      (Rendering|Material|SetScalarParameterValueonMaterials (Variables|Default|GetSphere) "Opacity" _newtrack_0))))

(fn ConstructionScript
  (Rendering|Material|SetScalarParameterValue "/Game/EasyDissolve/Materials/CollectionParameters/MPC_SphereMask.MPC_SphereMask" "Radius_1" (.X (Math|Vector|BreakVector (* (/ (Transformation|GetWorldScale (Variables|Default|GetSphere)) 2.0) 1e+02))) :!class /Script/Engine.KismetMaterialLibrary)
  (Rendering|Material|SetVectorParameterValue "/Game/EasyDissolve/Materials/CollectionParameters/MPC_SphereMask.MPC_SphereMask" "Location_1" (Math|Conversions|ToLinearColor(Vector) (Transformation|GetWorldLocation (Variables|Default|GetSphere))) :!class /Script/Engine.KismetMaterialLibrary))